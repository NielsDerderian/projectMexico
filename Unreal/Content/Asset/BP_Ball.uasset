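; BP_Ball is a physics ball that gets shot toward an end area, registering itself with the first-person game mode on BeginPlay.
; AddImpulseShot launches it with an acceleration-change force on its Sphere.
; A second sphere's overlaps with HOLE-tagged actors swap the Sphere's collision profile between Ball and BallHole.
; Whenever it moves, Tick sends its distance to the end area to the HUD as progression.
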(event OnComponentBeginOverlap(Sphere1)
  (params (OverlappedComponent :type Primitive%20Component%20Object%20Reference) (OtherActor :type Actor%20Object%20Reference) (OtherComp :type Primitive%20Component%20Object%20Reference) (OtherBodyIndex :type Integer) (bFromSweep :type Boolean) (SweepResult :type Hit%20Result%20Structure%20%28by%20ref%29))
  (if (Actor|ActorHasTag OtherActor "HOLE")
    (Collision|SetCollisionProfileName (Variables|Default|GetSphere) "BallHole" false :!class /Script/Engine.PrimitiveComponent)))

(event OnComponentEndOverlap(Sphere1)
  (params (OverlappedComponent :type Primitive%20Component%20Object%20Reference) (OtherActor :type Actor%20Object%20Reference) (OtherComp :type Primitive%20Component%20Object%20Reference) (OtherBodyIndex :type Integer))
  (if (Actor|ActorHasTag OtherActor "HOLE")
    (Collision|SetCollisionProfileName (Variables|Default|GetSphere) "Ball" true :!class /Script/Engine.PrimitiveComponent)))

(event Custom|SetupBallRef
  (params (Ref_HUD :type W%20HUD%20Object%20Reference) (Ref_EndArea :type BP%20Dynamic%20Hole%20Object%20Reference))
  (Variables|Default|SetRef%20HUD Ref_HUD)
  (Variables|Default|SetRef%20End%20Area Ref_EndArea))

(event EventBeginPlay
  (bind _asbp_first_person_game_mode (Utilities|Casting|CastToBP_FirstPersonGameMode (Game|GetGameMode)))
  (Default|UpdateBallRef _asbp_first_person_game_mode self))

(event EventTick
  (params (DeltaSeconds :type Float%20%28single-precision%29))
  (if (not (Utilities|Operators|EqualEqual (Transformation|GetActorLocation) (Variables|Default|GetlastLocation) 0.0))
    (Default|UpdateProgression (Variables|Default|GetRef%20HUD) (Math|Vector|VectorLength (- (Transformation|GetActorLocation) (Transformation|GetActorLocation (Variables|Default|GetRef%20End%20Area)))))
    (Variables|Default|SetlastLocation (Transformation|GetActorLocation))))

(event EventAddImpulseShot
  (params (Loc :type Vector :default "0, 0, 0") (Impulse :type Vector :default "0, 0, 0"))
  (Physics|AddForce (Variables|Default|GetSphere) Impulse "None" true))

(fn ConstructionScript)